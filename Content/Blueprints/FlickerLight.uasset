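; FlickerLight is an actor whose point light flickers on and off at random intervals, with a spark sound each time it relights.
; From BeginPlay an endless loop hides the light for a short random delay, then shows it and plays a fire-sparks cue at its location.
; The lit phase lasts a random time between MinFlickerTime and MaxFlickerTime, and the Volume variable scales the sound.
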(event `self.ReceiveBeginPlay`
  (`SceneComponent.SetVisibility` (`self.PointLight`) false false :!label _label)
  (`KismetSystemLibrary.RetriggerableDelay` (`KismetMathLibrary.RandomFloatInRange` 0.1 1.0))
  (`SceneComponent.SetVisibility` (`self.PointLight`) true false)
  (`GameplayStatics.SpawnSoundAtLocation` "/Game/StarterContent/Audio/Fire_Sparks01_Cue.Fire_Sparks01_Cue" (`SceneComponent.K2_GetComponentLocation` (`self.PointLight`)) (struct) (`self.Volume`) 1.0 0.0 null null)
  (`KismetSystemLibrary.RetriggerableDelay` (`KismetMathLibrary.RandomFloatInRange` (`self.MinFlickerTime`) (`self.MaxFlickerTime`)))
  (goto _label))

(fn `UserConstructionScript`)